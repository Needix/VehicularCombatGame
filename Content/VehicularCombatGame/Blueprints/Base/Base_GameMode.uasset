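; Base game mode for a vehicular combat game that sets up teams and spawns the player and AI cars at BeginPlay.
; Team actors spawn at random XY points between two LevelBoundary actors, raised above the first static hit of an upward vertical trace.
; The player possesses a car from the last team, then AI cars fill each team to capacity.
; A helper initializes ground particles on all drive pawns.
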(event EventBeginPlay
  (bind _teams (Variables|Team|GetTeams))
  (CallFunction|FindLevelBoundaries)
  (CallFunction|CreateTeams)
  (CallFunction|SpawnPlayer (Utilities|Array|Get(acopy) _teams (- (Utilities|Array|Length _teams) 1)))
  (CallFunction|SpawnAIs))

(fn ConstructionScript)

(fn FindLevelBoundaries
  (bind _outactors (Actor|GetAllActorsOfClass "/Game/VehicularCombatGame/Blueprints/AllLevel/LevelBoundary.LevelBoundary_C"))
  (if (== (Utilities|Array|Length _outactors) 2)
    (Variables|Boundary|SetLevelBoundary1 (Transformation|GetActorLocation (Utilities|Array|Get(acopy) _outactors)))
    (Variables|Boundary|SetLevelBoundary2 (Transformation|GetActorLocation (Utilities|Array|Get(acopy) _outactors 1)))))

(fn SpawnPlayer
  (params (Team :type Team%20Object%20Reference))
  (bind _returnvalue (Game|GetPlayerController 0))
  (bind _car (Default|SpawnCar Team _returnvalue "/Game/VehicularCombatGame/Blueprints/Player/Player_DriverPawn.Player_DriverPawn_C"))
  (Utilities|IsValid _car
    (:Is%20Valid
      (Pawn|Possess _returnvalue _car))))

(fn SpawnAIs
  (for _array_element (Variables|Team|GetTeams)
    (for _index (range (Utilities|Array|Length (Variables|/Game/VehicularCombatGame/Blueprints/GameModes/Team.Team_C|GetTeamPlayer _array_element)) (- (Variables|Team|GetMaxCarsPerTeam) 1))
      (bind _car (Default|SpawnCar _array_element 0 "/Game/VehicularCombatGame/Blueprints/AI/AI_DrivePawn.AI_DrivePawn_C"))
      (Utilities|IsValid _car
        (:Is%20Valid
          (Pawn|SpawnDefaultController _car))))))

(fn CreateTeams
  (bind _levelboundary1 (Variables|Boundary|GetLevelBoundary1))
  (bind _levelboundary2 (Variables|Boundary|GetLevelBoundary2))
  (bind (_x _y _z) (Math|Vector|BreakVector _levelboundary1))
  (bind (_x_2 _y_2 _z_2) (Math|Vector|BreakVector _levelboundary2))
  (for _index (range 0 (- (Variables|Team|GetMaxTeams) 1))
    (Variables|Default|SetlocX (Math|Random|RandomFloatinRange (Math|Float|Min(Float) _x _x_2) (Math|Float|Max(Float) _x _x_2)))
    (Variables|Default|SetlocY (Math|Random|RandomFloatinRange (Math|Float|Min(Float) _y _y_2) (Math|Float|Max(Float) _y _y_2)))
    (bind (_outhit _returnvalue) (Collision|LineTraceForObjects (Math|Vector|MakeVector (Variables|Default|GetlocX) (Variables|Default|GetlocY) -1e+08) (Math|Vector|MakeVector (Variables|Default|GetlocX) (Variables|Default|GetlocY) 1e+10) (Utilities|Array|MakeArray "ObjectTypeQuery1") false 0 "None"))
    (if _returnvalue
      (bind _returnvalue_2 (Game|SpawnActorfromClass "/Game/VehicularCombatGame/Blueprints/GameModes/Team.Team_C" (Math|Transform|MakeTransform (Math|Vector|MakeVector (Variables|Default|GetlocX) (Variables|Default|GetlocY) (+ (.Z (Math|Vector|BreakVector (.Location (Collision|BreakHitResult _outhit)))) 3e+02))) "AlwaysSpawn" 0 0))
      (Utilities|Array|Add (Variables|Team|GetTeams) _returnvalue_2))))

(fn InitAllParticles
  (params (Ground%20Particle%20System :type Particle%20System%20Object%20Reference))
  (bind _outactors (Actor|GetAllActorsOfClass "/Game/VehicularCombatGame/Blueprints/Base/Base_DrivePawn.Base_DrivePawn_C"))
  (for _array_element _outactors
    (Default|InitParticles _array_element Ground%20Particle%20System)))