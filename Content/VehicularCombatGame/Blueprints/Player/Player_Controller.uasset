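; Player controller for the vehicular combat game that respawns the player's car after death.
; Each tick, it checks whether player pawn 0 is valid and, if not, accumulates delta time.
; Once that timer reaches the game mode's death respawn time, it resets, has the Team spawn a driver pawn and possesses it.
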(event EventBeginPlay
  (bind _asbase_game_mode (Utilities|Casting|CastToBase_GameMode (Game|GetGameMode)))
  (Variables|Default|SetGameMode _asbase_game_mode))

(event EventTick
  (params (DeltaSeconds :type Float%20%28single-precision%29))
  (Variables|Default|SetDeltaSeconds DeltaSeconds)
  (CallFunction|CheckDeathCarRespawn))

(fn ConstructionScript)

(fn CheckDeathCarRespawn
  (Utilities|IsValid (Game|Player|GetPlayerPawn 0)
    (:Is%20Not%20Valid
      (Variables|CarRespawn|SetCarRespawnDeltaSeconds (+ (Variables|Default|GetDeltaSeconds) (Variables|CarRespawn|GetCarRespawnDeltaSeconds)))
      (if (>= (Variables|CarRespawn|GetCarRespawnDeltaSeconds) (Variables|/Game/VehicularCombatGame/Blueprints/Base/Base_GameMode.Base_GameMode_C|GetCONST_DeathRespawnTime (Variables|Default|GetGameMode)))
        (Variables|CarRespawn|SetCarRespawnDeltaSeconds 0.0)
        (bind _car (Default|SpawnCar (Variables|Team|GetTeam) self "/Game/VehicularCombatGame/Blueprints/Player/Player_DriverPawn.Player_DriverPawn_C"))
        (Pawn|Possess _car)))))