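; Team actor for the vehicular combat game that spawns cars for controllers and keeps track of them as team players.
; SpawnCar places the requested car class at a random horizontal offset around the actor's root, owned by the given controller, retrying if spawning fails.
; A successful spawn is added to TeamPlayer and returned, while exhausting the retries prints a warning.
; The event graph and construction script are empty.
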(event EventBeginPlay)

(event Collision|EventActorBeginOverlap
  (params (OtherActor :type Actor%20Object%20Reference)))

(event EventTick
  (params (DeltaSeconds :type Float%20%28single-precision%29)))

(fn ConstructionScript)

(fn SpawnCar
  (params (Controller :type Controller%20Object%20Reference) (Type :type Base%20Drive%20Pawn%20Class%20Reference))
  (bind _returnvalue (Math|Random|RandomFloatinRange -5e+02 5e+02))
  (bind _defaultsceneroot (Variables|Default|GetDefaultSceneRoot))
  (bind _returnvalue_2 (Transformation|GetWorldLocation _defaultsceneroot))
  (bind (_x _y _z) (Math|Vector|BreakVector _returnvalue_2))
  (Utilities|FlowControl|ForLoopwithBreak 0 10 :!label _label ; Try to spawn car 10 times
    (:LoopBody
      (bind _returnvalue_3 (Game|SpawnActorfromClass Type (Math|Conversions|ToTransform(Vector) (Math|Vector|MakeVector (+ _x _returnvalue) (+ _y _returnvalue) _z)) "Undefined" Controller 0))
      (Utilities|IsValid _returnvalue_3
        (:Is%20Valid
          (LocalVariables|SetResult _returnvalue_3)
          (LocalVariables|SetSuccessfull true)
          (goto _label Break))))
    (:Completed
      (if (LocalVariables|GetSuccessfull)
        (Utilities|Array|Add (Variables|Default|GetTeamPlayer) (LocalVariables|GetResult))
        (return (LocalVariables|GetResult))
        (else
          (Development|PrintString (Utilities|String|Append "WARNING: TeamBP: Could not spawn car after 10 tries. Parameters:" (Utilities|GetDisplayName Controller) " / " (Utilities|GetClassDisplayName Type))))))))