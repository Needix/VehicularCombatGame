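; AI-driven vehicle pawn that chases the closest player vehicle in the vehicular combat game.
; Each tick it scans all Player_DriverPawn actors for the nearest one, then releases the handbrake and drives toward it.
; Steering maps the yaw difference to the target onto steering input, and throttle rises with distance from a minimum to full, with no navmesh or obstacle avoidance.
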(event EventBeginPlay)

(event Collision|EventActorBeginOverlap
  (params (OtherActor :type Actor%20Object%20Reference)))

(event EventTick
  (params (DeltaSeconds :type Float%20%28single-precision%29))
  (|CallParentFunction DeltaSeconds)
  (CallFunction|FindClosestPlayer)
  (Utilities|IsValid (Variables|Default|GetClosestPlayer)
    (:Is%20Valid
      (Utilities|FlowControl|Sequence
        (:then_0
          (Class|WheeledVehicleMovementComponent|SetHandbrakeInput (Variables|Default|GetVehicleMovement) false))
        (:then_1
          (CallFunction|SetSteering))
        (:then_2
          (CallFunction|SetThrottle))))))

(fn ConstructionScript)

(fn FindClosestPlayer
  (bind _outactors (Actor|GetAllActorsOfClass "/Game/VehicularCombatGame/Blueprints/Player/Player_DriverPawn.Player_DriverPawn_C"))
  (for _array_element _outactors
    ;[1 1 1] Check all distances
    (if (or (== (LocalVariables|GetNearestPlayerDistance) 0.0) (>= (LocalVariables|GetNearestPlayerDistance) (Transformation|GetDistanceTo _array_element self)))
      (LocalVariables|SetNearestPlayerDistance (Transformation|GetDistanceTo _array_element self))
      (LocalVariables|SetNearestPlayer _array_element)))
  (Variables|Default|SetClosestPlayer (LocalVariables|GetNearestPlayer))
  (return))

(fn SetSteering
  (bind _mesh (Variables|Character|GetMesh))
  (Class|WheeledVehicleMovementComponent|SetSteeringInput (Variables|Default|GetVehicleMovement) (Math|Float|MapRangeClamped (.Yaw (Math|Rotator|BreakRotator (Math|Rotator|Delta(Rotator) (Math|Rotator|FindLookatRotation (Transformation|GetWorldLocation _mesh) (Transformation|GetWorldLocation (Variables|/Script/PhysXVehicles.WheeledVehicle|GetMesh (Variables|Default|GetClosestPlayer)))) (Transformation|GetWorldRotation _mesh)))) -1e+02 1e+02 -1.0 1.0)))

(fn SetThrottle
  (Class|WheeledVehicleMovementComponent|SetThrottleInput (Variables|Default|GetVehicleMovement) (Math|Float|MapRangeClamped (Transformation|GetDistanceTo (Variables|Default|GetClosestPlayer) self) 0.0 5e+03 0.3 1.0)))